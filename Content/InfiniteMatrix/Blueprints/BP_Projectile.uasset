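; BP_Projectile is a short-lived projectile that destroys enemies it overlaps.
; Each tick it moves along world X at ProjectileSpeed with a swept offset, and it destroys itself one second after spawning.
; On overlap it ignores other projectiles and the player, destroys a BP_Enemy along with itself, and destroys itself on any other actor.
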(event EventBeginPlay
  (Utilities|FlowControl|Delay 1.0)
  (Actor|DestroyActor))

(event Collision|EventActorBeginOverlap
  (params (OtherActor :type Actor%20Object%20Reference))
  (Utilities|Casting|CastToBP_Projectile OtherActor
    (:CastFailed
      (Utilities|Casting|CastToBP_Player OtherActor
        (:CastFailed
          (bind _asbp_enemy (Utilities|Casting|CastToBP_Enemy OtherActor)
            (:then
              (Actor|DestroyActor _asbp_enemy)
              (Actor|DestroyActor))
            (:CastFailed
              (Actor|DestroyActor))))))))

(event EventTick
  (params (DeltaSeconds :type Float%20%28single-precision%29))
  (Transformation|AddActorWorldOffset (Math|Vector|MakeVector (* DeltaSeconds (Variables|Default|GetProjectileSpeed)) 0.0 0.0) true))

(fn ConstructionScript)